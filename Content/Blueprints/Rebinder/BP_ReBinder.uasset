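; BP_ReBinder is a trigger-box actor that opens a rebinding UI when the player character walks into it.
; On begin overlap with BP_Character it creates WBP_Rebinding, adds it to the viewport, stores it and pauses the game.
; On end overlap it removes the widget, restores game-only input, hides the mouse cursor and re-enables character input, without unpausing the game itself.
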(event OnComponentBeginOverlap(Box)
  (params (OverlappedComponent :type Primitive%20Component%20Object%20Reference) (OtherActor :type Actor%20Object%20Reference) (OtherComp :type Primitive%20Component%20Object%20Reference) (OtherBodyIndex :type Integer) (bFromSweep :type Boolean) (SweepResult :type Hit%20Result%20Structure%20%28by%20ref%29))
  (Utilities|Casting|CastToBP_Character OtherActor)
  (bind _returnvalue (UserInterface|CreateWidget "/Game/Blueprints/UI/WBP_Rebinding.WBP_Rebinding_C"))
  (UserInterface|Viewport|AddtoViewport _returnvalue 0)
  (Variables|Default|SetWdiget _returnvalue)
  (Game|SetGamePaused true))

(event OnComponentEndOverlap(Box)
  (params (OverlappedComponent :type Primitive%20Component%20Object%20Reference) (OtherActor :type Actor%20Object%20Reference) (OtherComp :type Primitive%20Component%20Object%20Reference) (OtherBodyIndex :type Integer))
  (bind _returnvalue (Game|GetPlayerController 0))
  (bind _asbp_character (Utilities|Casting|CastToBP_Character OtherActor))
  (bind _wdiget (Variables|Default|GetWdiget)
    (:then
      (Input|SetInputModeGameOnly _returnvalue false)
      (Variables|/Script/Engine.PlayerController|SetbShowMouseCursor _returnvalue false)
      (Widget|RemovefromParent _wdiget)
      (Input|EnableInput _asbp_character _returnvalue))
    (:else)))

(event EventBeginPlay)

(event Collision|EventActorBeginOverlap
  (params (OtherActor :type Actor%20Object%20Reference)))

(event EventTick
  (params (DeltaSeconds :type Float%20%28single-precision%29)))

(fn ConstructionScript)